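; Win-condition volume that ends the game once every BP_Bunny in the level has been collected inside it.
; An overlapping bunny is detached from its controller and stopped, then all controllerless bunnies in the world are added uniquely to the collected array.
; When that array's length matches the total bunny count, it shows WBP_BunniesSaved and, after a short delay, opens the EndCredit level.
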(event `self.ReceiveBeginPlay`)

(event `self.ReceiveActorBeginOverlap`
  (params (OtherActor :type "Actor Object Reference"))
  (bind _asbp_bunny (cast `/Game/Blueprints/BP_Bunny` OtherActor))
  (`self.Disable Bunnies Overlapping and Add to Another Array` _asbp_bunny)
  (if (`self.AllBunniesCollected`)
    (bind _returnvalue (`|CreateWidget` "/Game/UI/WBP_BunniesSaved.WBP_BunniesSaved_C" (`GameplayStatics.GetPlayerController` 0)))
    (`UserWidget.AddToViewport` _returnvalue 0)
    (`KismetSystemLibrary.Delay` 3.0)
    (`GameplayStatics.OpenLevel` "EndCredit")))

(fn `AllBunniesCollected`
  (returns (ReturnValue :type Boolean))
  (bind _outactors (`GameplayStatics.GetAllActorsOfClass` "/Game/Blueprints/BP_Bunny.BP_Bunny_C"))
  (bind _output_get (set `self.RemainingBunniesInWorld` _outactors))
  (return (== (`KismetArrayLibrary.Array_Length` _output_get) (`KismetArrayLibrary.Array_Length` (`self.BunniesInWinVolumeDetachedFromAI`)))))

(fn `Disable Bunnies Overlapping and Add to Another Array`
  (params (Bunny :type "/Game/Blueprints/BP_Bunny Object Reference"))
  (`Pawn.DetachFromControllerPendingDestroy` Bunny)
  (`MovementComponent.StopMovementImmediately` (`Character.CharacterMovement` Bunny))
  (bind _outactors (`GameplayStatics.GetAllActorsOfClass` "/Game/Blueprints/BP_Bunny.BP_Bunny_C"))
  (bind _output_get (set `self.BunniesOverlapping` _outactors))
  (for _array_element _output_get
    (`/Engine/EditorBlueprintResources/StandardMacros.IsValid` (`Pawn.GetController` _array_element)
      (:`Is Not Valid`
        (`KismetArrayLibrary.Array_AddUnique` (`self.BunniesInWinVolumeDetachedFromAI`) _array_element)))))

(fn `UserConstructionScript`)