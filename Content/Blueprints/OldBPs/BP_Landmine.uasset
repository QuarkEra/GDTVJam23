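; BP_Landmine is a landmine actor that kills any BP_Bunny that overlaps it.
; On overlap it destroys the bunny, spawns explosion particles and sound, destroys itself and leaves smoke at its location.
; DoBunniesRemain sorts bunnies by valid controller to detect remaining ones, but only disconnected logic calls it.
; That unused logic would show the bunnies-saved widget, with a separate unused delayed jump to EndCredit.
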(event `self.ReceiveBeginPlay`)

(event `self.ReceiveActorBeginOverlap`
  (params (OtherActor :type "Actor Object Reference"))
  (bind _returnvalue (`self.K2_GetActorLocation`))
  ;[1 1 1] 1
  (bind _asbp_bunny (cast `/Game/Blueprints/OldBPs/BP_Bunny` OtherActor))
  (`self.K2_DestroyActor` _asbp_bunny)
  ;[1 1 1] 2
  (`GameplayStatics.SpawnEmitterAtLocation` "/Game/StarterContent/Particles/P_Explosion.P_Explosion" (`self.K2_GetActorLocation`))
  ;[1 1 1] 2
  (`GameplayStatics.PlaySoundAtLocation` "/Game/Audio/Explosion_Cue.Explosion_Cue" _returnvalue (struct) 1.0 1.0 0.0 null null null null)
  (`self.K2_DestroyActor`)
  ;[1 1 1] 3
  (`GameplayStatics.SpawnEmitterAtLocation` "/Game/StarterContent/Particles/P_Smoke.P_Smoke" _returnvalue))

(fn `DoBunniesRemain`
  (returns (`Return Value` :type Boolean))
  (bind _outactors (`GameplayStatics.GetAllActorsOfClass` "/Game/Blueprints/OldBPs/BP_Bunny.BP_Bunny_C"))
  (bind _output_get (set `self.BunniesRemaining` _outactors))
  (for _array_element _output_get
    (`/Engine/EditorBlueprintResources/StandardMacros.IsValid` (`Pawn.GetController` _array_element)
      (:`Is Valid`
        (`KismetArrayLibrary.Array_AddUnique` (`self.BunniesRemaining`) _array_element))
      (:`Is Not Valid`
        (`KismetArrayLibrary.Array_AddUnique` (`self.SavedBunnies`) _array_element))))
  (return (not (== (`KismetArrayLibrary.Array_Length` (`self.SavedBunnies`)) (`KismetArrayLibrary.Array_Length` (`self.BunniesRemaining`))))))

(fn `UserConstructionScript`)