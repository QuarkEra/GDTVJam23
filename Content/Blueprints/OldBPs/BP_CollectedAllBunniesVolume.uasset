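; Retired-looking win volume for collecting all bunnies, whose overlap logic is disconnected from its events, with a note mentioning C++.
; The unwired chain detaches a bunny's controller, stops its movement, and records every controllerless BP_Bunny in a unique array.
; When that array's count matches all bunnies in the world, it would show the WBP_BunniesSaved widget.
; A separate unwired chain would open EndCredit after a delay.
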(event `self.ReceiveBeginPlay`)

(event `self.ReceiveActorBeginOverlap`
  (params (OtherActor :type "Actor Object Reference")))

(fn `AllBunniesCollected`
  (returns (ReturnValue :type Boolean))
  (bind _outactors (`GameplayStatics.GetAllActorsOfClass` "/Game/Blueprints/OldBPs/BP_Bunny.BP_Bunny_C"))
  (bind _output_get (set `self.RemainingBunniesInWorld` _outactors))
  (return (== (`KismetArrayLibrary.Array_Length` _output_get) (`KismetArrayLibrary.Array_Length` (`self.BunniesInWinVolumeDetachedFromAI`)))))

(fn `Disable Bunnies Overlapping and Add to Another Array`
  (params (Bunny :type "/Game/Blueprints/OldBPs/BP_Bunny Object Reference"))
  (`Pawn.DetachFromControllerPendingDestroy` Bunny)
  (`MovementComponent.StopMovementImmediately` (`Character.CharacterMovement` Bunny))
  (bind _outactors (`GameplayStatics.GetAllActorsOfClass` "/Game/Blueprints/OldBPs/BP_Bunny.BP_Bunny_C"))
  (bind _output_get (set `self.BunniesOverlapping` _outactors))
  (for _array_element _output_get
    (`/Engine/EditorBlueprintResources/StandardMacros.IsValid` (`Pawn.GetController` _array_element)
      (:`Is Not Valid`
        (`KismetArrayLibrary.Array_AddUnique` (`self.BunniesInWinVolumeDetachedFromAI`) _array_element)))))

(fn `UserConstructionScript`)