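; Landmine actor that, when a BP_Bunny overlaps it, destroys the bunny and itself with explosion, sound and smoke effects.
; It then calls DoBunniesRemain, which adds bunnies without a valid controller to SavedBunnies and compares that count to all BP_Bunny actors.
; When the counts match, it shows the BunniesSaved widget and, after a Delay issued following its own DestroyActor, is set to open EndCredit.
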(event `self.ReceiveBeginPlay`)

(event `self.ReceiveActorBeginOverlap`
  (params (OtherActor :type "Actor Object Reference"))
  (bind _returnvalue (`self.K2_GetActorLocation`))
  (bind _asbp_bunny (cast `/Game/Blueprints/BP_Bunny` OtherActor))
  (`self.K2_DestroyActor` _asbp_bunny)
  (`GameplayStatics.SpawnEmitterAtLocation` "/Game/StarterContent/Particles/P_Explosion.P_Explosion" (`self.K2_GetActorLocation`))
  (`GameplayStatics.PlaySoundAtLocation` "/Game/StarterContent/Audio/Explosion_Cue.Explosion_Cue" _returnvalue (struct) 1.0 1.0 0.0 null null null null)
  (`self.K2_DestroyActor`)
  (`GameplayStatics.SpawnEmitterAtLocation` "/Game/StarterContent/Particles/P_Smoke.P_Smoke" _returnvalue)
  (bind _return_value (`self.DoBunniesRemain`))
  (if (not _return_value)
    (bind _returnvalue_2 (`|CreateWidget` "/Game/UI/WBP_BunniesSaved.WBP_BunniesSaved_C"))
    (`UserWidget.AddToViewport` _returnvalue_2 0)
    (`KismetSystemLibrary.Delay` 3.0)
    (`GameplayStatics.OpenLevel` "EndCredit")))

(fn `DoBunniesRemain`
  (returns (`Return Value` :type Boolean))
  (bind _outactors (`GameplayStatics.GetAllActorsOfClass` "/Game/Blueprints/BP_Bunny.BP_Bunny_C"))
  (bind _output_get (set `self.BunniesRemaining` _outactors))
  (for _array_element _output_get
    (`/Engine/EditorBlueprintResources/StandardMacros.IsValid` (`Pawn.GetController` _array_element)
      (:`Is Valid`
        (`KismetArrayLibrary.Array_AddUnique` (`self.BunniesRemaining`) _array_element))
      (:`Is Not Valid`
        (`KismetArrayLibrary.Array_AddUnique` (`self.SavedBunnies`) _array_element))))
  (return (not (== (`KismetArrayLibrary.Array_Length` (`self.SavedBunnies`)) (`KismetArrayLibrary.Array_Length` (`self.BunniesRemaining`))))))

(fn `UserConstructionScript`)